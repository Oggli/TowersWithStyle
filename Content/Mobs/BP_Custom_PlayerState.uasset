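; Custom PlayerState Blueprint that stores a player's economy and score stats: income, credits, lives and kills.
; Simple getter, setter and add functions read or change each variable, with kills only increasing one at a time and credits only changed by adding.
; It holds no event or construction logic, and nothing here applies income to credits or reacts to lives changing.
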(event EventBeginPlay)

(event EventTick
  (params (DeltaSeconds :type Float%20%28single-precision%29)))

(fn ConstructionScript)

(fn SetIncome
  (params (NewIncome :type Integer))
  (Variables|Default|SetIncome NewIncome))

(fn AddIncome
  (params (AdditionalIncome :type Integer))
  (Variables|Default|SetIncome (+ AdditionalIncome (Variables|Default|GetIncome))))

(fn GetIncome
  (return (Variables|Default|GetIncome)))

(fn AddCredits
  (params (CreditsToAdd :type Integer))
  (Variables|Default|SetCredits (+ CreditsToAdd (Variables|Default|GetCredits))))

(fn GetCredits
  (return (Variables|Default|GetCredits)))

(fn SetLives
  (params (NewTotalLives :type Integer))
  (Variables|Default|SetLives NewTotalLives))

(fn GetLives
  (return (Variables|Default|GetLives)))

(fn GetKills
  (return (Variables|Default|GetKills)))

(fn AddKill
  (Variables|Default|SetKills (+ (Variables|Default|GetKills) 1)))