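; Custom PlayerState for a wave-defense style game, tracking the player's credits, income, lives and kills.
; On BeginPlay it binds to every BP_MobSpawner, then hooks each newly spawned mob's destination-reached event.
; ProcessMobKill counts the kill and awards the mob's credit value, while PayCredits deducts a cost only when affordable.
; Life changes route through SetLives, which fires OnNoLivesLeft at zero or below.
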(event Custom|ProcessNewEnemy
  (params (MobSpawned :type BPA%20Mob%20Base%20Object%20Reference))
  (EventDispatchers|BindEventtoOnDestinationReached MobSpawned (EventDispatchers|CreateEvent :!event DecrementLives)))

(event EventBeginPlay
  (bind _outactors (Actor|GetAllActorsOfClass "/Game/Mobs/BP_MobSpawner.BP_MobSpawner_C"))
  (for _array_element _outactors
    (EventDispatchers|BindEventtoSpawnedNewUnit _array_element (delegate Custom|ProcessNewEnemy))))

(event EventTick
  (params (DeltaSeconds :type Float%20%28single-precision%29)))

(fn ConstructionScript)

(fn SetIncome
  (params (NewIncome :type Integer))
  (Variables|Default|SetIncome NewIncome))

(fn AddIncome
  (params (AdditionalIncome :type Integer))
  (Variables|Default|SetIncome (+ AdditionalIncome (Variables|Default|GetIncome))))

(fn GetIncome
  (return (Variables|Default|GetIncome)))

(fn AddCredits
  (params (CreditsToAdd :type Integer))
  (Variables|Default|SetCredits (+ CreditsToAdd (Variables|Default|GetCredits))))

(fn GetCredits
  (return (Variables|Default|GetCredits)))

(fn SetLives
  (params (NewTotalLives :type Integer))
  (bind _output_get (Variables|Default|SetLives NewTotalLives))
  (if (<= _output_get 0)
    (Default|CallOnNoLivesLeft)))

(fn GetLives
  (return (Variables|Default|GetLives)))

(fn GetKills
  (return (Variables|Default|GetKills)))

(fn AddKill
  (Math|Integer|IncrementInt (Variables|Default|GetKills)))

(fn PayCredits
  (params (Cost :type Integer))
  (if (<= Cost (Variables|Default|GetCredits))
    (Variables|Default|SetCredits (- (Variables|Default|GetCredits) Cost))
    (return true)
    (else
      (return false))))

(fn DecrementLives
  (bind _result (Math|Integer|DecrementInt (Variables|Default|GetLives))
    (:%20%20
      (CallFunction|SetLives _result))))

(fn ProcessMobKill
  (params (DeadMob :type BPA%20Mob%20Base%20Object%20Reference))
  (bind _newparam (Default|GetCreditValue DeadMob))
  (CallFunction|AddKill)
  (CallFunction|AddCredits _newparam))