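; BPC_Health is a health component that stores current and maximum HP and exposes getters for both.
; TakeDamage calls the OnDeath dispatcher when damage would bring HP to zero or below, leaving CurrentHP unchanged in that case.
; Otherwise it subtracts the damage and calls OnDamageTaken.
; BeginPlay and Tick are unused, so all logic runs through function calls.
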(event EventBeginPlay)

(event EventTick
  (params (DeltaSeconds :type Float%20%28single-precision%29)))

(fn GetHealth
  (return (Variables|Default|GetCurrentHP)))

(fn GetMaxHealth
  (return (Variables|Default|GetMaximumHP)))

(fn TakeDamage
  (params (Damage :type Integer))
  (if (<= (- (Variables|Default|GetCurrentHP) Damage) 0)
    (Default|CallOnDeath)
    (else
      (Variables|Default|SetCurrentHP (- (Variables|Default|GetCurrentHP) Damage))
      (Default|CallOnDamageTaken))))